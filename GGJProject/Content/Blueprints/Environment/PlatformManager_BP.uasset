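; Manager actor that collapses the level's FallingPlatform_BP platforms one by one, from the outside in.
; On BeginPlay it approximates their centre from summed locations divided by count plus one, then insertion-sorts them by squared distance from it.
; Tick runs a randomised short timer, enabling physics on the farthest remaining platform at each expiry.
; The timer stops when only the innermost platform remains.
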(event Custom|ResetTimer
  (Variables|Default|SetBreakingTimerMax (Math|Random|RandomFloatinRange 0.3 1.5))
  (Variables|Default|SetBreakingTimer 0.0))

(event EventBeginPlay
  (CallFunction|ResetTimer)
  (CallFunction|OrderPlatformsasDistancefromCentre)
  (Variables|Default|SetPlatformToFall (- (Utilities|Array|Length (Variables|Default|GetPlatforms)) 1))
  (Variables|Default|SetTimerActive true))

(event EventTick
  (params (DeltaSeconds :type Float%20%28single-precision%29))
  (if (Variables|Default|GetTimerActive)
    (bind _output_get (Variables|Default|SetBreakingTimer (+ DeltaSeconds (Variables|Default|GetBreakingTimer))))
    (if (>= _output_get (Variables|Default|GetBreakingTimerMax))
      (Physics|SetSimulatePhysics (Variables|/Game/Blueprints/Environment/FallingPlatform_BP.FallingPlatform_BP_C|GetPlatform (Utilities|Array|Get(acopy) (Variables|Default|GetPlatforms) (Variables|Default|GetPlatformToFall))) true)
      (bind _output_get_2 (Variables|Default|SetPlatformToFall (- (Variables|Default|GetPlatformToFall) 1)))
      (CallFunction|ResetTimer)
      (if (<= _output_get_2 0)
        (Variables|Default|SetTimerActive false)))))

(fn ConstructionScript)

(fn OrderPlatformsasDistancefromCentre
  (Utilities|FlowControl|Sequence
    (:then_0
      (bind _outactors (Actor|GetAllActorsOfClass "/Game/Blueprints/Environment/FallingPlatform_BP.FallingPlatform_BP_C"))
      (bind _output_get (LocalVariables|SetUnsortedPlatforms _outactors))
      (for _array_element _output_get
        (LocalVariables|SetPlatformsCentreLocation (+ (Transformation|GetWorldLocation (Variables|/Game/Blueprints/Environment/FallingPlatform_BP.FallingPlatform_BP_C|GetDefaultSceneRoot _array_element)) (LocalVariables|GetPlatformsCentreLocation))))
      (bind _output_get_2 (LocalVariables|SetPlatformsCentreLocation (/ (LocalVariables|GetPlatformsCentreLocation) (+ (Utilities|Array|Length (LocalVariables|GetUnsortedPlatforms)) 1))))
      (Development|PrintString (Utilities|String|ToString(Vector) _output_get_2) true true "(R=0.120157,G=1.000000,B=0.000000,A=1.000000)"))
    (:then_1
      (for (_array_element_2 _array_index) (LocalVariables|GetUnsortedPlatforms)
        (if (!= _array_index 0)
          (bind (_array_element_3 _array_index_2) (Utilities|Array|ForEachLoopwithBreak (Variables|Default|GetPlatforms) :!label _label)
            (:LoopBody
              (if (< (Math|Vector|VectorLengthSquared (- (Transformation|GetWorldLocation (Variables|/Game/Blueprints/Environment/FallingPlatform_BP.FallingPlatform_BP_C|GetDefaultSceneRoot _array_element_2)) (LocalVariables|GetPlatformsCentreLocation))) (Math|Vector|VectorLengthSquared (- (Transformation|GetWorldLocation (Variables|/Game/Blueprints/Environment/FallingPlatform_BP.FallingPlatform_BP_C|GetDefaultSceneRoot _array_element_3)) (LocalVariables|GetPlatformsCentreLocation))))
                (Utilities|Array|Insert (Variables|Default|GetPlatforms) _array_element_2 _array_index_2)
                (LocalVariables|SetAddedElementInLoop true)
                (goto _label Break)))
            (:Completed
              (if (LocalVariables|GetAddedElementInLoop)
                (LocalVariables|SetAddedElementInLoop false)
                (else
                  (Utilities|Array|Add (Variables|Default|GetPlatforms) _array_element_2)))))
          (else
            (Utilities|Array|Add (Variables|Default|GetPlatforms) _array_element_2)))))))