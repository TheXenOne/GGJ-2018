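; Blaster weapon actor that fires physics-driven projectiles from a barrel arrow for the UFO game demo.
; StartFire spawns a bullet immediately, then repeats SpawnBullet on a looping timer at the firing rate until EndFire clears it.
; Each bullet spawns at the arrow's transform, with the parent actor as owner and instigator, then gains forward velocity on its mesh.
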(event EventBeginPlay)

(event Collision|EventActorBeginOverlap
  (params (OtherActor :type Actor%20Object%20Reference)))

(event EventStartFire
  (Variables|Default|SetIsFiring true)
  (CallFunction|SpawnBullet)
  (Utilities|Time|SetTimerbyFunctionName 0 "SpawnBullet" (Variables|Default|GetFiring%20Rate) true))

(event EventTick
  (params (DeltaSeconds :type Float%20%28single-precision%29)))

(event EventEndFire
  (Variables|Default|SetIsFiring false)
  (Utilities|Time|ClearTimerbyFunctionName 0 "SpawnBullet"))

(fn ConstructionScript)

(fn NewFunction0)

(fn SpawnBullet
  (bind _returnvalue (Actor|GetParentActor))
  (bind _barrelarrow (Variables|Default|GetBarrelArrow))
  (bind _returnvalue_2 (Transformation|GetWorldTransform _barrelarrow))
  (bind _returnvalue_3 (Game|SpawnActorfromClass (Variables|Default|GetBullet%20Class) (Math|Transform|MakeTransform (.location _returnvalue_2) (.rotation _returnvalue_2) "1,1,1") "AlwaysSpawn" _returnvalue "/Engine/ArtTools/RenderToTexture/Meshes/S_1_Unit_Sphere.S_1_Unit_Sphere" 1.1 1.0 (.AsPawn (Utilities|Casting|CastToPawn _returnvalue))))
  (Physics|SetPhysicsLinearVelocity (Variables|/Game/UFOGameDemo/Weapons/BP_GameJamKit_Bullet_Actor.BP_GameJamKit_Bullet_Actor_C|GetMesh _returnvalue_3) (* (Math|Vector|GetForwardVector _barrelarrow) (Variables|Default|GetBullet%20Velocity)) true "None"))