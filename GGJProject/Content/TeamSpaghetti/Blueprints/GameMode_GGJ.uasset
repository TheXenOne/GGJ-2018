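; Game mode for a local multiplayer game that creates players and spawns their characters.
; On BeginPlay it caches all PlayerStarts and creates local players based on the game instance's NumPlayers.
; SpawnAllCharacters runs SpawnCharacter per controller, replacing any existing pawn with a Character_GGJ at a random, possibly shared, start.
; Each new character takes its controller ID as CharacterIndex and is possessed, with the view switched to the shared GameCamera.
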(event EventTick
  (params (DeltaSeconds :type Float%20%28single-precision%29)))

(event EventBeginPlay
  ;[1 1 1] Adds all the playerstarts to a spawn points array
  (bind _outactors (Actor|GetAllActorsOfClass "/Script/Engine.PlayerStart"))
  (Variables|Default|SetSpawnPoints _outactors)
  (bind _asgame_instance_ggj (Utilities|Casting|CastToGameInstance_GGJ (Game|GetGameInstance)))
  ;[1 1 1] Creates 4 players
  (for _index (range 0 (- (Variables|/Game/TeamSpaghetti/Blueprints/GameInstance_GGJ.GameInstance_GGJ_C|GetNumPlayers _asgame_instance_ggj) 1))
    (Class|GameplayStatics|CreatePlayer -1)))

(fn ConstructionScript)

(fn SpawnCharacter
  (params (PlayerController :type Player%20Controller%20Object%20Reference))
  (bind _returnvalue (Pawn|GetControlledPawn PlayerController))
  (bind _spawnpoints (Variables|Default|GetSpawnPoints))
  ;[1 1 1] Destroy old pawn
  (bind _output_get (LocalVariables|SetPlayer PlayerController))
  (Utilities|IsValid _returnvalue
    (:Is%20Valid
      (Actor|DestroyActor _returnvalue))
    (:Is%20Not%20Valid
      _))
  ;[1 1 1] Spawn new character and possess it
  (bind _returnvalue_2 (Game|SpawnActorfromClass "/Game/TeamSpaghetti/Blueprints/Character_GGJ.Character_GGJ_C" (Transformation|GetActorTransform (Utilities|Array|Get(acopy) _spawnpoints (Math|Random|RandomIntegerinRange 0 (Utilities|Array|LastIndex _spawnpoints)))) "AdjustIfPossibleButAlwaysSpawn" _output_get 0))
  (bind _returnvalue_3 (Class|GameplayStatics|GetPlayerControllerID (LocalVariables|GetPlayer)))
  (Variables|/Game/TeamSpaghetti/Blueprints/Character_GGJ.Character_GGJ_C|SetCharacterIndex _returnvalue_2 _returnvalue_3)
  (Development|PrintString (Utilities|GetDisplayName (LocalVariables|GetPlayer)))
  (Pawn|Possess (LocalVariables|GetPlayer) _returnvalue_2)
  ;[1 1 1] Sets camera to proper camera set in level
  (Game|Player|SetViewTargetwithBlend (LocalVariables|GetPlayer) (Variables|Default|GetGameCamera) 0.0 "VTBlend_Linear" 0.0 false))

(fn SpawnAllCharacters
  (bind _asgame_instance_ggj (Utilities|Casting|CastToGameInstance_GGJ (Game|GetGameInstance)))
  (for _index (range 0 (- (Variables|/Game/TeamSpaghetti/Blueprints/GameInstance_GGJ.GameInstance_GGJ_C|GetNumPlayers _asgame_instance_ggj) 1))
    (CallFunction|SpawnCharacter (Game|GetPlayerController _index))))