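; Player character for a multiplayer slime brawler, with five size stages that set speed, turning, jump and acceleration while a timeline lerps scale.
; Jumping can become a cooldown-gated butt stomp that spawns a size-aware shockwave on landing.
; Sprinting shows player-colored particles that leave splat decals and enables knockback bumps.
; Punch input only sets flags; the Punch function steals size on hit or sheds a projectile on miss.
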(event OnComponentHit(CapsuleComponent)
  (params (HitComponent :type Primitive%20Component%20Object%20Reference) (OtherActor :type Actor%20Object%20Reference) (OtherComp :type Primitive%20Component%20Object%20Reference) (NormalImpulse :type Vector :default "0, 0, 0") (Hit :type Hit%20Result%20Structure%20%28by%20ref%29))
  (bind _ascharacter_ggj (Utilities|Casting|CastToCharacter_GGJ OtherActor))
  (CallFunction|BumpIntoPlayer (.impactnormal Hit) _ascharacter_ggj))

(event Custom|On%20Collide%20Event
  (params (EventName :type Name) (EmitterTime :type Float%20%28single-precision%29) (ParticleTime :type Integer) (Location :type Vector) (Velocity :type Vector) (Direction :type Vector) (Normal :type Vector) (BoneName :type Name) (PhysMat :type Physical%20Material%20Object%20Reference))
  (bind _returnvalue (Math|Random|RandomFloatinRange 1e+02 2.5e+02))
  (Rendering|Decal|SpawnDecalatLocation (Variables|Default|GetSplatMaterialInstance) (Math|Vector|MakeVector 1.0 _returnvalue _returnvalue) Location (Math|Conversions|RotationFromXVector (* Normal -1.0)) 2e+01))

(event Custom|SizeChangeEvent_Event
  ;[1 1 1] ScaleChangeEvent
  (bind _lerp (Timeline|LerpScaleTimeline PlayFromStart)
    (:Update
      (Transformation|SetActorScale3D (Math|Vector|Lerp(Vector) (Variables|Default|GetTempScaleVariable) (Utilities|Array|Get(acopy) (Variables|DesignersFap|GetStagesScaleValues) (Variables|Default|GetCurrentStage)) _lerp)))))

(event EventBeginPlay
  (bind _playercolor (Variables|Default|GetPlayerColor))
  (EventDispatchers|BindEventtoSizeChangeEvent (delegate Custom|SizeChangeEvent_Event))
  (Variables|Default|SetCurrentStage 2)
  (CallFunction|UpdateStage)
  (Variables|Default|SetButtStompTimerTimer (Variables|DesignersFap|GetButtStompCooldown))
  (Effects|Components|ParticleSystem|SetVectorParameter (Variables|Default|GetParticleSystem) "TrailColor" (Math|Vector|MakeVector (.r _playercolor) (.g _playercolor) (.b _playercolor)))
  (EventDispatchers|BindEventtoOnParticleCollide (Variables|Default|GetParticleSystem) (delegate Custom|On%20Collide%20Event))
  (bind _returnvalue (Rendering|Material|CreateDynamicMaterialInstance "/Game/TeamSpaghetti/Blueprints/Particles/Blood_Decal_Mat.Blood_Decal_Mat" :!class /Script/Engine.KismetMaterialLibrary))
  (Rendering|Material|SetScalarParameterValue _returnvalue "Frame" (Math|Conversions|ToFloat(Integer) (Math|Random|RandomInteger 11)) :!class /Script/Engine.MaterialInstanceDynamic)
  (Rendering|Material|SetVectorParameterValue _returnvalue "GoopColor" (Variables|Default|GetPlayerColor) :!class /Script/Engine.MaterialInstanceDynamic)
  (Variables|Default|SetSplatMaterialInstance _returnvalue))

(event Collision|EventActorBeginOverlap
  (params (OtherActor :type Actor%20Object%20Reference)))

(event EventTick
  (params (DeltaSeconds :type Float%20%28single-precision%29))
  (Variables|Default|SetDeltaTime DeltaSeconds)
  (Utilities|FlowControl|Sequence
    (:then_0
      (bind _output_get (Variables|Default|SetButtStompTimerTimer (+ (Variables|Default|GetButtStompTimerTimer) (Variables|Default|GetDeltaTime))))
      (if (>= _output_get (Variables|DesignersFap|GetButtStompCooldown))
        (if (Variables|Default|GetIsJumping)
          (if (< (.z (Transformation|GetVelocity)) (Variables|DesignersFap|GetButtStompThresholdValue))
            (Variables|Default|SetCanButtStomp true)))))
    (:then_1
      (CallFunction|HandleSprint))))

(event EventOnLanded
  (params (Hit :type Hit%20Result%20Structure%20%28by%20ref%29))
  ;[1 1 1] Jumping and ButtStomping
  (Variables|Default|SetIsJumping false)
  (Variables|Default|SetCanButtStomp false)
  (if (Variables|Default|GetIsButtstomping)
    (Variables|Default|SetIsButtstomping false)
    (CallFunction|CreateShockwave)))

(event Input|ActionEvents|InputActionScaleUp
  (params (Key :type Key%20Structure))
  (:Pressed
    (CallFunction|Grow)))

(event Input|ActionEvents|InputActionScaleDown
  (params (Key :type Key%20Structure))
  (:Pressed
    (CallFunction|Shrink)))

(event Input|ActionEvents|InputActionJumpEvent
  (params (Key :type Key%20Structure))
  ;[1 1 1] Jumping and ButtStomping
  (:Pressed
    (if (Variables|Default|GetIsJumping)
      (if (Variables|Default|GetCanButtStomp)
        (CallFunction|ButtStomp)
        (Variables|Default|SetButtStompTimerTimer 0.0))
      (else
        (Character|Jump)
        (Variables|Default|SetIsJumping true)))))

(event Input|ActionEvents|InputActionPunch
  (params (Key :type Key%20Structure))
  (:Pressed
    (CallFunction|PunchNew)))

(event Input|AxisEvents|InputAxisWalkForward
  (params (AxisValue :type Float%20%28single-precision%29))
  (bind _returnvalue (Transformation|GetActorLocation))
  ;[1 1 1] Walking
  (Pawn|Input|AddMovementInput "1.000000, 0,0.000000" AxisValue false)
  ;[1 1 1] Rotating/Aiming
  (if (> (Math|Vector|VectorLength (Math|Vector|MakeVector AxisValue (stale Input|AxisEvents|InputAxisWalkSide AxisValue) 0.0)) 0.0)
    (Pawn|SetControlRotation (Game|GetPlayerController (Variables|Default|GetCharacterIndex)) (Math|Interpolation|RInterpTo (Transformation|GetActorRotation) (Math|Rotator|FindLookatRotation _returnvalue (+ (Math|Vector|MakeVector AxisValue (stale Input|AxisEvents|InputAxisWalkSide AxisValue) 0.0) _returnvalue)) (Variables|Default|GetDeltaTime) (Variables|Default|GetRotInterpSpeed)))))

(event Input|AxisEvents|InputAxisLookForward
  (params (AxisValue :type Float%20%28single-precision%29))
  ;[1 1 1] Rotating/Aiming
)

(event Input|AxisEvents|InputAxisLookSide
  (params (AxisValue :type Float%20%28single-precision%29))
  ;[1 1 1] Rotating/Aiming
)

(event Input|AxisEvents|InputAxisWalkSide
  (params (AxisValue :type Float%20%28single-precision%29))
  (bind _returnvalue (Transformation|GetActorLocation))
  ;[1 1 1] Walking
  (Pawn|Input|AddMovementInput "0,1.000000,0.000000" AxisValue false)
  ;[1 1 1] Rotating/Aiming
  (if (> (Math|Vector|VectorLength (Math|Vector|MakeVector (stale Input|AxisEvents|InputAxisWalkForward AxisValue) AxisValue 0.0)) 0.0)
    (Pawn|SetControlRotation (Game|GetPlayerController (Variables|Default|GetCharacterIndex)) (Math|Interpolation|RInterpTo (Transformation|GetActorRotation) (Math|Rotator|FindLookatRotation _returnvalue (+ (Math|Vector|MakeVector (stale Input|AxisEvents|InputAxisWalkForward AxisValue) AxisValue 0.0) _returnvalue)) (Variables|Default|GetDeltaTime) (Variables|Default|GetRotInterpSpeed)))))

(event Input|GamepadEvents|GamepadSpecialRight
  (params (Key :type Key%20Structure))
  (bind _returnvalue (Game|GetPlayerController 0))
  ;[1 1 1] Pause Screen
  (:Pressed
    (Utilities|IsValid (Variables|Default|GetPause%20Menu%20Reference)
      (:Is%20Valid
        (Input|SetInputModeGameandUI _returnvalue 0 "DoNotLock" true)
        (UserInterface|Viewport|AddtoViewport (Variables|Default|GetPause%20Menu%20Reference) 0)
        (Game|SetGamePaused true)
        (Variables|/Script/Engine.PlayerController|SetbShowMouseCursor _returnvalue true))
      (:Is%20Not%20Valid
        (bind _returnvalue_2 (UserInterface|CreateWidget "/Game/TeamSpaghetti/Blueprints/UI/PauseMenu.PauseMenu_C"))
        (Variables|Default|SetPause%20Menu%20Reference _returnvalue_2)))))

(fn ConstructionScript)

(fn Grow
  (if (< (Variables|Default|GetCurrentStage) 4)
    (Math|Integer|IncrementInt (Variables|Default|GetCurrentStage)
      (:%20%20
        (CallFunction|UpdateStage)
        (return true)))
    (else
      (return false))))

(fn Shrink
  (if (> (Variables|Default|GetCurrentStage) 0)
    (Math|Integer|DecrementInt (Variables|Default|GetCurrentStage)
      (:%20%20
        (CallFunction|UpdateStage)
        (return true)))
    (else
      (return false))))

(fn UpdateStage
  (Variables|Default|SetTempScaleVariable (Transformation|GetActorScale3D))
  (Variables|/Script/Engine.CharacterMovementComponent|SetMaxWalkSpeed (Variables|Character|GetCharacterMovement) (Utilities|Array|Get(acopy) (Variables|DesignersFap|GetStagesMovementSpeed) (Variables|Default|GetCurrentStage)))
  (Variables|Default|SetRotInterpSpeed (Utilities|Array|Get(acopy) (Variables|DesignersFap|GetStagesRotationSpeed) (Variables|Default|GetCurrentStage)))
  (Variables|/Script/Engine.CharacterMovementComponent|SetJumpZVelocity (Variables|Character|GetCharacterMovement) (Utilities|Array|Get(acopy) (Variables|DesignersFap|GetStagesJumpingForce) (Variables|Default|GetCurrentStage)))
  (Variables|/Script/Engine.CharacterMovementComponent|SetMaxAcceleration (Variables|Character|GetCharacterMovement) (Utilities|Array|Get(acopy) (Variables|DesignersFap|GetStagesAcceleration) (Variables|Default|GetCurrentStage)))
  (Default|CallSizeChangeEvent))

(fn ButtStomp
  (Variables|Default|SetCanButtStomp false)
  (Components|Movement|StopMovementImmediately (Variables|Character|GetCharacterMovement))
  (Physics|AddImpulse (Variables|Character|GetCharacterMovement) "0, 0,-100000.000000" false)
  (Variables|Default|SetIsButtstomping true))

(fn CreateShockwave
  (bind _returnvalue (Game|SpawnActorfromClass "/Game/TeamSpaghetti/Blueprints/ShockwaveRing.ShockwaveRing_C" (Math|Transform|MakeTransform (Transformation|GetWorldLocation (Variables|Default|GetShockwaveSpawnPoint)) "0, 0, 0" "1,1,1") "AlwaysSpawn" 0 self (Utilities|Array|Get(acopy) (Variables|DesignersFap|GetStagesButtstompPushingForce) (Variables|Default|GetCurrentStage)) (Variables|Default|GetPlayerColor) 0))
  (Variables|/Game/TeamSpaghetti/Blueprints/ShockwaveRing.ShockwaveRing_C|SetSpawningActorSize _returnvalue (Variables|Default|GetCurrentStage)))

(fn Punch
  (bind _punchdistance (Variables|DesignersFap|GetPunchDistance))
  (bind _punchspawnpoint (Variables|Default|GetPunchSpawnPoint))
  (bind _returnvalue (Transformation|GetWorldLocation _punchspawnpoint))
  (bind _returnvalue_2 (Math|Vector|GetForwardVector _punchspawnpoint))
  (bind _returnvalue_3 (* _returnvalue_2 _punchdistance))
  (bind _returnvalue_4 (+ _returnvalue _returnvalue_3))
  (LocalVariables|SetLaunchDirection (Math|Vector|Normalize (- _returnvalue_4 _returnvalue)))
  (bind (_outhit _returnvalue_5) (Collision|LineTraceByChannel _returnvalue _returnvalue_4 "TraceTypeQuery1" false 0 "None"))
  (if _returnvalue_5
    ;[1 1 1] If something is hit, punch
    (bind _ascharacter_ggj (Utilities|Casting|CastToCharacter_GGJ (.HitActor (Collision|BreakHitResult _outhit))))
    (Character|LaunchCharacter _ascharacter_ggj (* (Math|Vector|RotateVectorAroundAxis (.ImpactNormal (Collision|BreakHitResult _outhit)) 1.8e+02 "0, 0,1.000000") (Utilities|Array|Get(acopy) (Variables|DesignersFap|GetStagesButtstompPushingForce) (Variables|Default|GetCurrentStage))) true true)
    (CallFunction|Shrink _ascharacter_ggj)
    (CallFunction|Grow)
    (else
      (CallFunction|LoseMass (LocalVariables|GetLaunchDirection)))))

(fn AdjustStage
  (params (StageChange :type Integer))
  (Variables|Default|SetCurrentStage (Math|Integer|Clamp(Integer) (+ StageChange (Variables|Default|GetCurrentStage)) 0 4))
  (CallFunction|UpdateStage))

(fn HandleSprint
  (bind _returnvalue (Transformation|GetVelocity))
  (bind _output_get (Variables|Default|SetIsSprinting (>= (Math|Vector|VectorLength (Math|Vector|MakeVector (.x _returnvalue) (.y _returnvalue) 0.0)) (Utilities|Array|Get(acopy) (Variables|DesignersFap|GetStagesMinimumSprintSpeed) (Variables|Default|GetCurrentStage)))))
  (Rendering|SetVisibility (Variables|Default|GetParticleSystem) _output_get false))

(fn LoseMass
  (params (LaunchDirection :type Vector))
  ;[1 1 1] If miss, lose mass
  (bind _succeeded (CallFunction|Shrink))
  (if _succeeded
    (Game|SpawnActorfromClass "/Game/TeamSpaghetti/Blueprints/Pickups/SlimeProjectile_BP.SlimeProjectile_BP_C" (Math|Transform|MakeTransform (Transformation|GetWorldLocation (Variables|Default|GetPunchSpawnPoint)) "0, 0, 0" "1,1,1") "AlwaysSpawn" 0 LaunchDirection (Variables|Default|GetPlayerColor) self)))

(fn BumpIntoPlayer
  (params (HitImpactNormal :type Vector) (HitPlayer :type Character%20GGJ%20Object%20Reference))
  (bind _returnvalue (* HitImpactNormal -1.0))
  (bind _stagessprintpushingforce (Variables|DesignersFap|GetStagesSprintPushingForce))
  (bind _currentstage (Variables|Default|GetCurrentStage))
  (bind _output (Utilities|Array|Get(acopy) _stagessprintpushingforce _currentstage))
  (bind _returnvalue_2 (* _returnvalue _output))
  ;[1 1 1] Launch character away from hitting player in the direction they were hit from
  (if (Variables|Default|GetIsSprinting)
    (Character|LaunchCharacter HitPlayer (Math|Vector|MakeVector (.x _returnvalue_2) (.y _returnvalue_2) 2.5e+02) true true)
    ;[1 1 1] Pushes the pushing character back a bit based on how hard they hit the enemy player
    (Character|LaunchCharacter (Math|Vector|MakeVector (* (* (.y _returnvalue_2) 0.7) -1.0) (* (* (.x _returnvalue_2) 0.7) -1.0) 1e+02) true true)))

(fn RotateParticles
  (Transformation|SetWorldRotation (Variables|Default|GetParticleSystem) (Math|Rotator|MakeRotfromX (* (Math|Vector|Normalize (Transformation|GetVelocity)) -1.0)) false false))

(fn PunchNew
  (if (and (Variables|Default|GetCanPunch) (not (Variables|Default|GetIsJumping)))
    (Variables|Default|SetIsPunching true)
    (Variables|Default|SetCanPunch false)))