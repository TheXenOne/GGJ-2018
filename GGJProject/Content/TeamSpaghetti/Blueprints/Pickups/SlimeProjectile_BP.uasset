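; SlimeProjectile_BP is a colored slime projectile that leaves a pickup and a splat where it lands on a falling platform.
; Construction sets its velocity from VelocityDir and tints a dynamic ToxicWater material with MaterialColor.
; Hitting either falling platform type spawns a SlimePickup_BP in that color, adds a randomly sized, temporary decal using the instigating Character_GGJ's splat material, then destroys the projectile.
; Other hits are ignored.
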(event OnComponentHit(Sphere)
  (params (HitComponent :type Primitive%20Component%20Object%20Reference) (OtherActor :type Actor%20Object%20Reference) (OtherComp :type Primitive%20Component%20Object%20Reference) (NormalImpulse :type Vector :default "0, 0, 0") (Hit :type Hit%20Result%20Structure%20%28by%20ref%29))
  (bind (_bblockinghit _binitialoverlap _time _distance _location _impactpoint _normal) (Collision|BreakHitResult Hit))
  (bind _returnvalue (Math|Random|RandomFloatinRange 1e+02 2.5e+02))
  (bind (_x _y _z) (Math|Vector|BreakVector _location))
  (Utilities|Casting|CastToFallingPlatform_BP OtherActor
    (:then
      _)
    (:CastFailed
      (Utilities|Casting|CastToFallingPlatformSetTime_BP OtherActor)))
  (Game|SpawnActorfromClass "/Game/TeamSpaghetti/Blueprints/Pickups/SlimePickup_BP.SlimePickup_BP_C" (Math|Transform|MakeTransform _location "0, 0, 0" "1,1,1") "AlwaysSpawn" 0 (Variables|Default|GetMaterialColor) 0)
  (bind _ascharacter_ggj (Utilities|Casting|CastToCharacter_GGJ (Game|GetInstigator)))
  (Rendering|Decal|SpawnDecalatLocation (Variables|/Game/TeamSpaghetti/Blueprints/Character_GGJ.Character_GGJ_C|GetSplatMaterialInstance _ascharacter_ggj) (Math|Vector|MakeVector 1.0 _returnvalue _returnvalue) (Math|Vector|MakeVector _x _y (- _z 5.0)) (Math|Conversions|RotationFromXVector (* _normal -1.0)) 2e+01)
  (Actor|DestroyActor))

(event EventBeginPlay)

(event Collision|EventActorBeginOverlap
  (params (OtherActor :type Actor%20Object%20Reference)))

(event EventTick
  (params (DeltaSeconds :type Float%20%28single-precision%29)))

(fn ConstructionScript
  (Variables|/Script/Engine.MovementComponent|SetVelocity (Variables|Default|GetProjectileMovement) (Variables|Default|GetVelocityDir))
  (bind _returnvalue (Rendering|Material|CreateDynamicMaterialInstance "/Game/Art/Materials/ToxicWater.ToxicWater" :!class /Script/Engine.KismetMaterialLibrary))
  (bind _output_get (Variables|Default|SetMaterialReference _returnvalue))
  (Rendering|Material|SetVectorParameterValue _output_get "Color" (Variables|Default|GetMaterialColor) :!class /Script/Engine.MaterialInstanceDynamic)
  (Rendering|Material|SetMaterial (Variables|Default|GetStaticMesh) 0 (Variables|Default|GetMaterialReference)))