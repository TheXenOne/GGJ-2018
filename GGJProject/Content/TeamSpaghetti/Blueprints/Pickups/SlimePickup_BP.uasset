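; Slime pickup Blueprint that makes the player character grow when touched.
; On actor overlap it casts to Character_GGJ, calls Grow on it and destroys itself.
; The construction script creates a dynamic ToxicWater material instance, sets its Color from the MaterialColor variable and applies it to the Sphere, allowing a color per instance.
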(event EventBeginPlay)

(event Collision|EventActorBeginOverlap
  (params (OtherActor :type Actor%20Object%20Reference))
  (bind _ascharacter_ggj (Utilities|Casting|CastToCharacter_GGJ OtherActor))
  (Default|Grow _ascharacter_ggj)
  (Actor|DestroyActor))

(event EventTick
  (params (DeltaSeconds :type Float%20%28single-precision%29)))

(fn ConstructionScript
  (bind _returnvalue (Rendering|Material|CreateDynamicMaterialInstance "/Game/Art/Materials/ToxicWater.ToxicWater" :!class /Script/Engine.KismetMaterialLibrary))
  (bind _output_get (Variables|Default|SetMaterialReference _returnvalue))
  (Rendering|Material|SetVectorParameterValue _output_get "Color" (Variables|Default|GetMaterialColor) :!class /Script/Engine.MaterialInstanceDynamic)
  (Rendering|Material|SetMaterial (Variables|Default|GetSphere) 0 (Variables|Default|GetMaterialReference)))