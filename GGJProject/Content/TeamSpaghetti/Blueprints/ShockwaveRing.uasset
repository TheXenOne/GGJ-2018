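; Shockwave ring actor that knocks other characters away from its center, sized by the spawning character's current stage.
; On BeginPlay a timeline scales the ring to that stage's max scale, then destroys it, alongside a stomp particle matched in radius and player color.
; Overlapped characters, except the spawner, are launched radially outward, tilted 45 degrees upward.
; The construction script tints the plane through a dynamic material using the shockwave color.
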(event EventBeginPlay
  (Variables|Default|SetSpawningActorSize (Variables|/Game/TeamSpaghetti/Blueprints/Character_GGJ.Character_GGJ_C|GetCurrentStage (Variables|Default|GetSpawningActor)))
  (Utilities|FlowControl|Sequence
    (:then_0
      (bind _scale (Timeline|Scale PlayFromStart)
        (:Update
          (Transformation|SetActorScale3D (Math|Vector|Lerp(Vector) "1.000000,1.000000,1.000000" (Utilities|Array|Get(acopy) (Variables|DesignerFap|GetMaxScale) (Variables|Default|GetSpawningActorSize)) _scale)))
        (:Finished
          (Actor|DestroyActor))))
    (:then_1
      (bind _returnvalue (Effects|SpawnEmitteratLocation "/Game/TeamSpaghetti/Blueprints/Particles/P_Stomp.P_Stomp" (Transformation|GetActorLocation) "0, 0, 0" (/ (Utilities|Array|Get(acopy) (Variables|DesignerFap|GetMaxScale) (Variables|Default|GetSpawningActorSize)) 1e+01)))
      (Effects|Components|ParticleSystem|SetFloatParameter _returnvalue "Radius" (Utilities|Array|Get(acopy) (Variables|DesignerFap|GetParticleRadiuses) (Variables|Default|GetSpawningActorSize)))
      (Effects|Components|ParticleSystem|SetColorParameter _returnvalue "Color" (Variables|/Game/TeamSpaghetti/Blueprints/Character_GGJ.Character_GGJ_C|GetPlayerColor (Variables|Default|GetSpawningActor))))))

(event Collision|EventActorBeginOverlap
  (params (OtherActor :type Actor%20Object%20Reference))
  (bind _returnvalue (Transformation|GetActorLocation))
  (bind _ascharacter_ggj (Utilities|Casting|CastToCharacter_GGJ OtherActor))
  (if (!= _ascharacter_ggj (Variables|Default|GetSpawningActor))
    (Character|LaunchCharacter _ascharacter_ggj (Math|Vector|RotateVectorAroundAxis (* (Math|Vector|Normalize (- (Math|Vector|MakeVector (.x (Transformation|GetActorLocation _ascharacter_ggj)) (.y (Transformation|GetActorLocation _ascharacter_ggj)) 0.0) (Math|Vector|MakeVector (.x _returnvalue) (.y _returnvalue) 0.0))) (Variables|Default|GetPushingStrenght)) -45.0 (Math|Vector|RotateVectorAroundAxis (* (Math|Vector|Normalize (- (Math|Vector|MakeVector (.x (Transformation|GetActorLocation _ascharacter_ggj)) (.y (Transformation|GetActorLocation _ascharacter_ggj)) 0.0) (Math|Vector|MakeVector (.x _returnvalue) (.y _returnvalue) 0.0))) (Variables|Default|GetPushingStrenght)) 9e+01 "0, 0,1.000000")) true true)))

(event EventTick
  (params (DeltaSeconds :type Float%20%28single-precision%29)))

(fn ConstructionScript
  (bind _returnvalue (Rendering|Material|CreateDynamicMaterialInstance "/Game/TeamSpaghetti/Assets/ExplosionTemp_Mat.ExplosionTemp_Mat" :!class /Script/Engine.KismetMaterialLibrary))
  (bind _output_get (Variables|Default|SetMaterialReference _returnvalue))
  (Rendering|Material|SetVectorParameterValue _output_get "Color" (Variables|Default|GetShockwaveColor) :!class /Script/Engine.MaterialInstanceDynamic)
  (Rendering|Material|SetMaterial (Variables|Default|GetPlane) 0 (Variables|Default|GetMaterialReference)))