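; Falling platform actor that drops after a set amount of time once its timer is active.
; Each tick, while TimerActive is true, it accumulates delta seconds into a break timer.
; When the timer reaches TimeUntilPlatformBreaks, it enables physics simulation on the Platform component so it falls, then stops the timer.
; Nothing in this graph sets TimerActive to true.
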(event EventTick
  (params (DeltaSeconds :type Float%20%28single-precision%29))
  (if (Variables|Default|GetTimerActive)
    (bind _output_get (Variables|Default|SetPlatformBreakTimer (+ (Variables|Default|GetPlatformBreakTimer) DeltaSeconds)))
    (if (>= _output_get (Variables|Default|GetTimeUntilPlatformBreaks))
      (Physics|SetSimulatePhysics (Variables|Default|GetPlatform) true)
      (Variables|Default|SetTimerActive false))))

(fn ConstructionScript)