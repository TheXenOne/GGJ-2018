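; Manager that makes the level's falling platforms drop one at a time, from the outermost inward, and registers itself with GameMode_GGJ.
; On BeginPlay it averages all platform locations into a centre and insertion-sorts those flagged to fall by squared distance from it.
; While enabled, Tick runs a random or fixed countdown, applies a danger material to the next platform, then enables its physics after a warning delay.
; It also activates separate set-time platform timers once.
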(event Custom|ResetTimer
  ;[1 1 1] Reset Timer
  (if (Variables|DesignerFAP|GetUseRandomPlatformBreakTime)
    (Variables|BreakingTimerNOEDIT|SetBreakingTimerMax (Math|Random|RandomFloatinRange (Variables|DesignerFAP|GetPlatformBreakTimeMin) (Variables|DesignerFAP|GetPlatformBreakTimeMax)))
    (else
      (Variables|BreakingTimerNOEDIT|SetBreakingTimerMax (Variables|DesignerFAP|GetBreakTimeNoRandom))))
  (Variables|BreakingTimerNOEDIT|SetBreakingTimer 0.0))

(event EventBeginPlay
  (bind _asgame_mode_ggj (Utilities|Casting|CastToGameMode_GGJ (Game|GetGameMode)))
  (Variables|/Game/TeamSpaghetti/Blueprints/GameMode_GGJ.GameMode_GGJ_C|SetPlatformManager _asgame_mode_ggj self)
  (CallFunction|ResetTimer)
  (CallFunction|OrderPlatformsasDistancefromCentre)
  (Variables|BreakingTimerNOEDIT|SetPlatformToFall (- (Utilities|Array|Length (Variables|BreakingTimerNOEDIT|GetPlatforms)) 1))
  (bind _outactors (Actor|GetAllActorsOfClass "/Game/TeamSpaghetti/Blueprints/Environment/FallingPlatformSetTime_BP.FallingPlatformSetTime_BP_C"))
  (Variables|BreakingTimerNOEDIT|SetFallingPlatformsSetTimers _outactors)
  (Variables|BreakingTimerNOEDIT|SetTimerActive true))

(event EventTick
  (params (DeltaSeconds :type Float%20%28single-precision%29))
  (if (Variables|Default|GetEnabled?)
    ;[1 1 1] Platform Falling Timer
    (if (Variables|BreakingTimerNOEDIT|GetTimerActive)
      (Utilities|FlowControl|Sequence
        (:then_0
          (Utilities|FlowControl|DoOnce false
            (:Completed
              (for _array_element (Variables|BreakingTimerNOEDIT|GetFallingPlatformsSetTimers)
                (Variables|/Game/TeamSpaghetti/Blueprints/Environment/FallingPlatformSetTime_BP.FallingPlatformSetTime_BP_C|SetTimerActive _array_element true)))))
        (:then_1
          _))
      (bind _output_get (Variables|BreakingTimerNOEDIT|SetBreakingTimer (+ DeltaSeconds (Variables|BreakingTimerNOEDIT|GetBreakingTimer))))
      (if (>= _output_get (Variables|BreakingTimerNOEDIT|GetBreakingTimerMax))
        ;[1 1 1] Platform Fall, Reset Timer
        (CallFunction|PlatformFalling (Variables|/Game/TeamSpaghetti/Blueprints/Environment/FallingPlatform_BP.FallingPlatform_BP_C|GetPlatform (Utilities|Array|Get(acopy) (Variables|BreakingTimerNOEDIT|GetPlatforms) (Variables|BreakingTimerNOEDIT|GetPlatformToFall))))
        (bind _output_get_2 (Variables|BreakingTimerNOEDIT|SetPlatformToFall (- (Variables|BreakingTimerNOEDIT|GetPlatformToFall) 1)))
        (CallFunction|ResetTimer)
        ;[1 1 1] Stop when on last platform
        (if (<= _output_get_2 -1)
          (Variables|BreakingTimerNOEDIT|SetTimerActive false))))))

(fn ConstructionScript)

(fn OrderPlatformsasDistancefromCentre
  (Utilities|FlowControl|Sequence
    (:then_0
      ;[1 1 1] Get platforms centre location
      (bind _outactors (Actor|GetAllActorsOfClass "/Game/TeamSpaghetti/Blueprints/Environment/FallingPlatform_BP.FallingPlatform_BP_C"))
      (bind _output_get (LocalVariables|SetUnsortedPlatforms _outactors))
      (for _array_element _output_get
        (LocalVariables|SetPlatformsCentreLocation (+ (Transformation|GetWorldLocation (Variables|/Game/TeamSpaghetti/Blueprints/Environment/FallingPlatform_BP.FallingPlatform_BP_C|GetDefaultSceneRoot _array_element)) (LocalVariables|GetPlatformsCentreLocation))))
      (bind _output_get_2 (LocalVariables|SetPlatformsCentreLocation (/ (LocalVariables|GetPlatformsCentreLocation) (Utilities|Array|Length (LocalVariables|GetUnsortedPlatforms)))))
      (Development|PrintString (Utilities|String|ToString(Vector) _output_get_2) false true "(R=0.120157,G=1.000000,B=0.000000,A=1.000000)"))
    (:then_1
      ;[1 1 1] Loop through Unsorted Platforms, then looping through platforms, inserting unsorted platforms by distance from centre location
      (for _array_element_2 (LocalVariables|GetUnsortedPlatforms)
        (bind (_array_element_3 _array_index) (Utilities|Array|ForEachLoopwithBreak (Variables|BreakingTimerNOEDIT|GetPlatforms) :!label _label)
          (:LoopBody
            (if (and (< (Math|Vector|VectorLengthSquared (- (Transformation|GetWorldLocation (Variables|/Game/TeamSpaghetti/Blueprints/Environment/FallingPlatform_BP.FallingPlatform_BP_C|GetDefaultSceneRoot _array_element_2)) (LocalVariables|GetPlatformsCentreLocation))) (Math|Vector|VectorLengthSquared (- (Transformation|GetWorldLocation (Variables|/Game/TeamSpaghetti/Blueprints/Environment/FallingPlatform_BP.FallingPlatform_BP_C|GetDefaultSceneRoot _array_element_3)) (LocalVariables|GetPlatformsCentreLocation)))) (Variables|/Game/TeamSpaghetti/Blueprints/Environment/FallingPlatform_BP.FallingPlatform_BP_C|GetFalls _array_element_2))
              (Utilities|Array|Insert (Variables|BreakingTimerNOEDIT|GetPlatforms) _array_element_2 _array_index)
              (LocalVariables|SetAddedElementInLoop true)
              (goto _label Break)))
          (:Completed
            (if (LocalVariables|GetAddedElementInLoop)
              (LocalVariables|SetAddedElementInLoop false)
              (elif (Variables|/Game/TeamSpaghetti/Blueprints/Environment/FallingPlatform_BP.FallingPlatform_BP_C|GetFalls _array_element_2)
                (Utilities|Array|Add (Variables|BreakingTimerNOEDIT|GetPlatforms) _array_element_2)
                (else
                  (Variables|BreakingTimerNOEDIT|SetNumberNotFalling (+ (Variables|BreakingTimerNOEDIT|GetNumberNotFalling) 1)))))))))))

(fn PlatformFalling
  (params (Platform :type Static%20Mesh%20Component%20Object%20Reference))
  (Rendering|Material|SetMaterial Platform 0 "/Game/Art/Art/Materials/MeshMaterials/M_Dangerous.M_Dangerous")
  (bind _asfalling_platform_bp (Utilities|Casting|CastToFallingPlatform_BP (Components|GetOwner Platform)))
  (Utilities|Time|SetTimerbyFunctionName _asfalling_platform_bp "SetPhysicsEnabled" (Variables|DesignerFAP|GetWarningTime)))