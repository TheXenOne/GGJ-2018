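; Shared multiplayer camera that becomes the first player controller's view target and keeps all active characters framed.
; Each Tick finds the farthest-apart pair, lerps toward their midpoint, and sets spring arm length from their distance plus a player-count buffer, clamped to minimum zoom.
; Players below a Z threshold are dropped; a lone survivor gets a close follow, and with none left it drifts to the origin.
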(event Custom|AddPlayers
  ;[1 1 1] Check for player character actors > 0
  (bind _outactors (Actor|GetAllActorsOfClass "/Game/TeamSpaghetti/Blueprints/Character_GGJ.Character_GGJ_C"))
  (if (!= (Utilities|Array|Length _outactors) 0)
    (bind _outactors_2 (Actor|GetAllActorsOfClass "/Game/TeamSpaghetti/Blueprints/Character_GGJ.Character_GGJ_C"))
    (Variables|CameraNOEDIT|SetPlayers _outactors_2)
    (bind _outactors_3 (Actor|GetAllActorsOfClass "/Game/TeamSpaghetti/Blueprints/PlayerController_GGJ.PlayerController_GGJ_C"))
    (bind _output_get (Variables|CameraNOEDIT|SetPlayerController (Utilities|Array|Get(acopy) _outactors_3)))
    (Game|Player|SetViewTargetwithBlend _output_get self 0.0 "VTBlend_Linear" 0.0 false)
    (Variables|CameraNOEDIT|SetPlayerPresent true)
    (Development|PrintString (Utilities|String|ToString(Integer) (Utilities|Array|Length (Variables|CameraNOEDIT|GetPlayers))) false)
    (else
      (Transformation|SetActorLocation "0, 0, 0" false false))))

(event Custom|WinnerCamera
  (Transformation|SetActorLocation (Math|Vector|Lerp(Vector) (Transformation|GetActorLocation) (Transformation|GetActorLocation (Utilities|Array|Get(acopy) (Variables|CameraNOEDIT|GetPlayers))) 0.05) false false)
  (Variables|/Script/Engine.SpringArmComponent|SetTargetArmLength (Variables|Default|GetSpringArm) (Math|Float|Lerp (Variables|/Script/Engine.SpringArmComponent|GetTargetArmLength (Variables|Default|GetSpringArm)) (Variables|DesignerFAP|GetMinimumZoom) 0.3)))

(event Custom|CheckFallenPlayers
  ;[1 1 1] Check for fallen players to ignore
  (for _array_element (Variables|CameraNOEDIT|GetPlayers)
    (if (<= (.z (Transformation|GetActorLocation _array_element)) (Variables|DesignerFAP|GetZIgnore))
      (Utilities|Array|RemoveItem (Variables|CameraNOEDIT|GetPlayers) _array_element))))

(event EventBeginPlay
  ;[1 1 1] At start try to add players
  (CallFunction|AddPlayers))

(event EventTick
  (params (DeltaSeconds :type Float%20%28single-precision%29))
  (bind _players (Variables|CameraNOEDIT|GetPlayers))
  (bind _returnvalue (Utilities|Array|Length _players))
  ;[1 1 1] If players more than 1, execute sequence, if 1 player, focus on them, if none, centre camera
  (if (Variables|CameraNOEDIT|GetPlayerPresent)
    (if (> _returnvalue 1)
      (Utilities|FlowControl|Sequence
        (:then_0
          ;[1 1 1] Loop through all players with nested for, finding largest distance between them O(n^2)
          (Variables|CameraNOEDIT|SetMidpoint "0, 0, 0")
          (for (_array_element _array_index) (Variables|CameraNOEDIT|GetPlayers)
            (for (_array_element_2 _array_index_2) (Variables|CameraNOEDIT|GetPlayers)
              (if (!= _array_index_2 _array_index)
                (Development|PrintString "Hello" false false)
                (if (> (Math|Vector|VectorLength (- (Transformation|GetActorLocation _array_element_2) (Transformation|GetActorLocation _array_element))) (Variables|CameraNOEDIT|GetLargestDistance))
                  (Variables|CameraNOEDIT|SetLargestDistance (Math|Vector|VectorLength (- (Transformation|GetActorLocation _array_element_2) (Transformation|GetActorLocation _array_element))))
                  (Variables|CameraNOEDIT|SetMidpoint (+ (/ (- (Transformation|GetActorLocation _array_element_2) (Transformation|GetActorLocation _array_element)) 2.0) (Transformation|GetActorLocation _array_element))))))))
        (:then_1
          ;[1 1 1] Lerp to midpoint between furthest players
          (Transformation|SetActorLocation (Math|Vector|Lerp(Vector) (Transformation|GetActorLocation) (Variables|CameraNOEDIT|GetMidpoint) 0.05) false false)
          ;[1 1 1] Check < min zoom distance
          (CallFunction|CalculateBufferMultiplier (Utilities|Array|Length (Variables|CameraNOEDIT|GetPlayers)))
          (if (<= (Math|Float|Lerp (Variables|/Script/Engine.SpringArmComponent|GetTargetArmLength (Variables|Default|GetSpringArm)) (+ (Variables|CameraNOEDIT|GetLargestDistance) (* (Variables|DesignerFAP|GetBuffer) (Variables|CameraNOEDIT|GetBufferMult))) 0.3) (Variables|DesignerFAP|GetMinimumZoom))
            ;[1 1 1] Set target arm length
            (Variables|/Script/Engine.SpringArmComponent|SetTargetArmLength (Variables|Default|GetSpringArm) (Math|Float|Lerp (Variables|/Script/Engine.SpringArmComponent|GetTargetArmLength (Variables|Default|GetSpringArm)) (Variables|DesignerFAP|GetMinimumZoom) 0.3))
            (else
              (Variables|/Script/Engine.SpringArmComponent|SetTargetArmLength (Variables|Default|GetSpringArm) (Math|Float|Lerp (Variables|/Script/Engine.SpringArmComponent|GetTargetArmLength (Variables|Default|GetSpringArm)) (+ (Variables|CameraNOEDIT|GetLargestDistance) (* (Variables|DesignerFAP|GetBuffer) (Variables|CameraNOEDIT|GetBufferMult))) 0.3))))
          (Variables|CameraNOEDIT|SetC1Dist "0, 0, 0")
          (Variables|CameraNOEDIT|SetLargestDistance 0.0))
        (:then_2
          ;[1 1 1] Call CheckFallenPlayers
          (CallFunction|CheckFallenPlayers)))
      (elif (== _returnvalue 1)
        (CallFunction|WinnerCamera)
        (CallFunction|CheckFallenPlayers)
        (else
          (Transformation|SetActorLocation (Math|Vector|Lerp(Vector) (Transformation|GetActorLocation) "0, 0, 0" 0.05) false false)
          (Variables|/Script/Engine.SpringArmComponent|SetTargetArmLength (Variables|Default|GetSpringArm) (Math|Float|Lerp (Variables|/Script/Engine.SpringArmComponent|GetTargetArmLength (Variables|Default|GetSpringArm)) (Variables|DesignerFAP|GetMinimumZoom) 0.3)))))
    (else
      (CallFunction|AddPlayers))))

(fn ConstructionScript)

(fn CalculateBufferMultiplier
  (params (NumPlayers :type Integer))
  (if (== NumPlayers 2)
    (Variables|CameraNOEDIT|SetBufferMult (Variables|DesignerFAP|GetBufferMult2Players))
    (elif (== NumPlayers 3)
      (Variables|CameraNOEDIT|SetBufferMult (Variables|DesignerFAP|GetBufferMult3Players))
      (elif (== NumPlayers 4)
        (Variables|CameraNOEDIT|SetBufferMult (Variables|DesignerFAP|GetBufferMult4Players))))))